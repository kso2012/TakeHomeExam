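; Hero_BP is a player-controlled hero that spawns a gun, moves, and turns with separate input axes.
; On BeginPlay it spawns Gun_BP and attaches it to the mesh's GunPoint socket.
; MoveForward and MoveRight add movement along fixed world X and Y axes.
; TurnForward and Turn share logic that sets facing from an axis-built direction vector, ignoring near-zero input.
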(event `self.ReceiveBeginPlay`
  (bind _returnvalue (`|SpawnActorFromClass` "/Game/Gun/Gun_BP.Gun_BP_C" (`self.GunPosition`) "Undefined" "OverrideRootScale"))
  (`self.K2_AttachToComponent` _returnvalue (`self.Mesh`) "GunPoint" "KeepRelative" "KeepRelative" "KeepRelative" true))

(event `InputAxis|MoveForward`
  (params (AxisValue :type "Float (single-precision)"))
  (`self.AddMovementInput` (1.0 0.0 0.0) AxisValue))

(event `InputAxis|MoveRight`
  (params (AxisValue :type "Float (single-precision)"))
  (`self.AddMovementInput` (0.0 1.0 0.0) AxisValue))

(event `InputAxis|TurnForward`
  (params (AxisValue :type "Float (single-precision)"))
  (bind _returnvalue (`KismetMathLibrary.MakeVector` AxisValue (stale `InputAxis|Turn` AxisValue)))
  (if (not (`KismetMathLibrary.NearlyEqual_FloatFloat` (`KismetMathLibrary.VSizeSquared` _returnvalue) 0.0 0.01)) :!label _label
    (`self.K2_SetActorRotation` (`KismetMathLibrary.Conv_VectorToRotator` _returnvalue))))

(event `InputAxis|Turn`
  (params (AxisValue :type "Float (single-precision)"))
  (goto _label))

(fn `UserConstructionScript`)